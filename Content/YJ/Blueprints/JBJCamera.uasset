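; JBJCamera is a camera actor with an unfinished check for whether it is looking at the player.
; Each Tick it runs a Visibility line trace 2000 units along the camera's forward vector, drawn for debugging, and casts the hit to BP_Player and a BoxComponent.
; Nothing follows the casts: the camera location and rotation setters and an impact-distance test are left unconnected, so the trace has no gameplay effect.
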(event EventBeginPlay)

(event Collision|EventActorBeginOverlap
  (params (OtherActor :type Actor%20Object%20Reference)))

(event EventTick
  (params (DeltaSeconds :type Float%20%28single-precision%29))
  (bind _camera (Variables|Default|GetCamera))
  (bind _returnvalue (Transformation|GetWorldLocation _camera))
  (bind _outhit (Collision|LineTraceByChannel _returnvalue (+ _returnvalue (* (Math|Vector|GetForwardVector _camera) 2e+03)) "TraceTypeQuery1" false 0 "ForOneFrame" true "(R=1.000000,G=0.000000,B=0.000000,A=1.000000)" "(R=0.000000,G=1.000000,B=0.000000,A=1.000000)" 1.0))
  (Utilities|Casting|CastToBP_Player (.hitactor _outhit))
  (Utilities|Casting|CastToBoxComponent (.hitcomponent _outhit)))

(fn ConstructionScript)