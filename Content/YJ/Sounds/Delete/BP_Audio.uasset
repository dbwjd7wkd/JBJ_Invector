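; BP_Audio is an audio visualization actor that plays its Audio component on BeginPlay and scales meshes in response to playback.
; The single envelope value uniformly scales the Sphere, while the playback percent stretches the Cylinder along Z.
; Each playback update also calculates a short frequency spectrum of a hard-coded Avicii track at the current game time, but the result is unused.
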(event OnAudioSingleEnvelopeValue(Audio)
  (params (PlayingSoundWave :type Sound%20Wave%20Object%20Reference) (EnvelopeValue :type Float%20%28single-precision%29))
  (Transformation|SetRelativeScale3D (Variables|Default|GetSphere) (Math|Conversions|ToVector(Float) (* EnvelopeValue 1e+01))))

(event OnAudioPlaybackPercent(Audio)
  (params (PlayingSoundWave :type Sound%20Wave%20Object%20Reference) (PlaybackPercent :type Float%20%28single-precision%29))
  (Transformation|SetRelativeScale3D (Variables|Default|GetCylinder) (Math|Vector|MakeVector 1.0 1.0 (* PlaybackPercent 5.0)))
  (Class|SoundVisualizationStatics|CalculateFrequencySpectrum "/Game/YJ/Sounds/Avicii_Heaven_wav.Avicii_Heaven_wav" 0 (Utilities|Time|GetGameTimeinSeconds) 0.08 10))

(event EventBeginPlay
  (Audio|Components|Audio|Play (Variables|Default|GetAudio) 0.0))

(fn ConstructionScript)