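; Audio visualizer Blueprint that plays the Avicii Heaven track as 2D sound and shows a WBP_Play widget.
; On each playback-percent update, it calculates the frequency spectrum at the current playback time.
; Each spectrum value's scaled magnitude is written to all four progress bars, so they end up showing the last value.
; An unconnected branch holds code for building a row of cube meshes from the spectrum.
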(event OnAudioPlaybackPercent(Audio)
  (params (PlayingSoundWave :type Sound%20Wave%20Object%20Reference) (PlaybackPercent :type Float%20%28single-precision%29))
  (bind _main (Variables|Default|GetMain))
  (Utilities|IsValid (Variables|Default|GetAudio)
    (:Is%20Valid
      (bind _outspectrum (Class|SoundVisualizationStatics|CalculateFrequencySpectrum "/Game/YJ/Sounds/Avicii_Heaven_wav.Avicii_Heaven_wav" 0 (* (Variables|/Script/Engine.SoundBase|GetDuration (Variables|/Script/Engine.AudioComponent|GetSound (Variables|Default|GetAudio))) PlaybackPercent) 0.08 (Variables|Default|GetSpectrum%20Width)))
      (for _array_element _outspectrum
        (Utilities|FlowControl|Sequence
          (:then_0
            (Progress|SetPercent (Variables|/Game/YJ/GUI/WBP_Play.WBP_Play_C|GetProgressBar_1 _main) (/ (Math|Float|Absolute(Float) _array_element) 5e+01)))
          (:then_1
            (Progress|SetPercent (Variables|/Game/YJ/GUI/WBP_Play.WBP_Play_C|GetProgressBar_2 _main) (/ (Math|Float|Absolute(Float) _array_element) 5e+01)))
          (:then_2
            (Progress|SetPercent (Variables|/Game/YJ/GUI/WBP_Play.WBP_Play_C|GetProgressBar_3 _main) (/ (Math|Float|Absolute(Float) _array_element) 5e+01)))
          (:then_3
            (Progress|SetPercent (Variables|/Game/YJ/GUI/WBP_Play.WBP_Play_C|GetProgressBar_4 _main) (/ (Math|Float|Absolute(Float) _array_element) 5e+01))))))))

(event EventBeginPlay
  (bind _returnvalue (UserInterface|CreateWidget "/Game/YJ/GUI/WBP_Play.WBP_Play_C"))
  (bind _output_get (Variables|Default|SetMain _returnvalue))
  (UserInterface|Viewport|AddtoViewport _output_get 0)
  (bind _returnvalue_2 (Audio|SpawnSound2D "/Game/YJ/Sounds/Avicii_Heaven_wav.Avicii_Heaven_wav" 1.0 1.0 0.0 0))
  (Variables|Default|SetAudio _returnvalue_2))

(fn ConstructionScript)