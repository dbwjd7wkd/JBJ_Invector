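; BP_Audio_2 is an audio visualizer actor that plays the Avicii Heaven track and shows its frequency spectrum as a row of cubes.
; On BeginPlay it starts the audio and creates one non-simulated cube mesh per spectrum band, spaced along X and stored in MeshArray.
; On each playback-percent update it recalculates the spectrum at the current song position and scales each cube's height by that band's absolute amplitude.
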(event OnAudioPlaybackPercent(Audio)
  (params (PlayingSoundWave :type Sound%20Wave%20Object%20Reference) (PlaybackPercent :type Float%20%28single-precision%29))
  (bind _outspectrum (Class|SoundVisualizationStatics|CalculateFrequencySpectrum "/Game/YJ/Sounds/Avicii_Heaven_wav.Avicii_Heaven_wav" 0 (* (Variables|/Script/Engine.SoundBase|GetDuration (Variables|/Script/Engine.AudioComponent|GetSound (Variables|Default|GetAudio))) PlaybackPercent) 0.08 (Variables|Default|GetSpectrum%20Width)))
  (for (_array_element _array_index) _outspectrum
    (Transformation|SetRelativeScale3D (Utilities|Array|Get(acopy) (Variables|Default|GetMeshArray) _array_index) (Math|Vector|MakeVector 0.4 0.4 (/ (Math|Float|Absolute(Float) _array_element) 1e+01)))))

(event EventBeginPlay
  (bind _returnvalue (Math|Vector|MakeVector -2.5e+02 0.0 0.0))
  (Audio|Components|Audio|Play (Variables|Default|GetAudio) 0.0)
  (bind _outspectrum (Class|SoundVisualizationStatics|CalculateFrequencySpectrum "/Game/YJ/Sounds/Avicii_Heaven_wav.Avicii_Heaven_wav" 0 0.0 0.08 (Variables|Default|GetSpectrum%20Width)))
  (for (_ _array_index) _outspectrum
    (bind _returnvalue_2 (AddComponent|AddStaticMeshComponent false (Math|Transform|MakeTransform (Math|Vector|MakeVector (+ (* (Math|Conversions|ToFloat(Integer) _array_index) 5e+01) (.x _returnvalue)) (.y _returnvalue) (.z _returnvalue)) "0, 0, 0" "0.400000,0.400000,0.400000")))
    (Components|StaticMesh|SetStaticMesh _returnvalue_2 "/Game/Geometry/Meshes/1M_Cube.1M_Cube")
    (Utilities|Array|SetArrayElem (Variables|Default|GetMeshArray) _array_index _returnvalue_2 true)
    (Physics|SetSimulatePhysics _returnvalue_2 false)))

(fn ConstructionScript)