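; BP_PlayUI_Audio_Manager shows the play UI and drives an audio-reactive meter on it from the music's amplitude.
; BeginPlay creates the WBP_Play widget, adds it to the viewport, then starts the Audio component after a short delay.
; The component's single-envelope-value event normalizes and doubles the amplitude, floors it at a small minimum, and applies that same value to all ten progress bars in the widget.
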(event OnAudioSingleEnvelopeValue(Audio)
  (params (PlayingSoundWave :type Sound%20Wave%20Object%20Reference) (EnvelopeValue :type Float%20%28single-precision%29))
  (bind _returnvalue (Math|Float|NormalizetoRange EnvelopeValue 0.0 1.0))
  (bind _main (Variables|Default|GetMain))
  (bind _returnvalue_2 (* _returnvalue 2.0))
  (if (> _returnvalue_2 0.1)
    (Variables|Default|SetPercent _returnvalue_2)
    (else
      (Variables|Default|SetPercent 0.1)))
  (Utilities|FlowControl|Sequence
    (:then_0
      (Progress|SetPercent (Variables|/Game/YJ/GUI/WBP_Play.WBP_Play_C|GetProgressBar _main) (Variables|Default|GetPercent)))
    (:then_1
      (Progress|SetPercent (Variables|/Game/YJ/GUI/WBP_Play.WBP_Play_C|GetProgressBar_1 _main) (Variables|Default|GetPercent)))
    (:then_2
      (Progress|SetPercent (Variables|/Game/YJ/GUI/WBP_Play.WBP_Play_C|GetProgressBar_2 _main) (Variables|Default|GetPercent)))
    (:then_3
      (Progress|SetPercent (Variables|/Game/YJ/GUI/WBP_Play.WBP_Play_C|GetProgressBar_3 _main) (Variables|Default|GetPercent)))
    (:then_4
      (Progress|SetPercent (Variables|/Game/YJ/GUI/WBP_Play.WBP_Play_C|GetProgressBar_4 _main) (Variables|Default|GetPercent)))
    (:then_5
      (Progress|SetPercent (Variables|/Game/YJ/GUI/WBP_Play.WBP_Play_C|GetProgressBar_5 _main) (Variables|Default|GetPercent)))
    (:then_6
      (Progress|SetPercent (Variables|/Game/YJ/GUI/WBP_Play.WBP_Play_C|GetProgressBar_6 _main) (Variables|Default|GetPercent)))
    (:then_7
      (Progress|SetPercent (Variables|/Game/YJ/GUI/WBP_Play.WBP_Play_C|GetProgressBar_7 _main) (Variables|Default|GetPercent)))
    (:then_8
      (Progress|SetPercent (Variables|/Game/YJ/GUI/WBP_Play.WBP_Play_C|GetProgressBar_8 _main) (Variables|Default|GetPercent)))
    (:then_9
      (Progress|SetPercent (Variables|/Game/YJ/GUI/WBP_Play.WBP_Play_C|GetProgressBar_9 _main) (Variables|Default|GetPercent)))))

(event EventBeginPlay
  (bind _returnvalue (UserInterface|CreateWidget "/Game/YJ/GUI/WBP_Play.WBP_Play_C"))
  (bind _output_get (Variables|Default|SetMain _returnvalue))
  (UserInterface|Viewport|AddtoViewport _output_get 0)
  (Utilities|FlowControl|Delay 3.7)
  (Audio|Components|Audio|Play (Variables|Default|GetAudio) 0.0))

(fn ConstructionScript)